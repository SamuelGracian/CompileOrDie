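; Player spaceship for a Starfox-style game that flies along a level spline on a timed rail.
; On BeginPlay it finds the tagged BP_SplinePath and registers the Enhanced Input mapping context.
; A timeline, rate-scaled by TimeToComplete, lerps distance along the spline and sets the ship's location and rotation each update.
; IA_Movement separately adds movement input along control-rotation right and forward vectors.
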(event Custom|Spline%20movement
  (bind _spline_to_follow (Variables|Default|GetSpline%20to%20follow))
  (bind _spline (Variables|/Game/Starfox/BluePrints/BP_SplinePath.BP_SplinePath_C|GetSpline _spline_to_follow))
  (Components|Timeline|SetPlayRate (Variables|Default|GetTimeline) (/ 1.0 (Variables|Default|GetTime%20to%20complete)))
  (bind _flight_track (Timeline|Timeline Play)
    (:Update
      (Transformation|SetActorLocationAndRotation (Spline|GetLocationatDistanceAlongSpline _spline (Math|Float|Lerp 0.0 (Spline|GetSplineLength _spline) _flight_track) "World") (Spline|GetRotationatDistanceAlongSpline _spline (Math|Float|Lerp 0.0 (Spline|GetSplineLength _spline) _flight_track) "Local")))))

(event Input|EnhancedActionEvents|EnhancedInputActionIA_Movement
  (params (ActionValue :type Vector%202D%20Structure) (ElapsedSeconds :type Float%20%28double-precision%29) (TriggeredSeconds :type Float%20%28double-precision%29) (InputAction :type Input%20Action%20Object%20Reference :default "/Game/Starfox/Inputs/Input_actions/IA_Movement.IA_Movement"))
  (bind _returnvalue (Pawn|GetControlRotation :!class /Script/Engine.Pawn))
  (Pawn|Input|AddMovementInput (Math|Vector|GetRightVector (Math|Rotator|MakeRotator (.roll _returnvalue) 0.0 (.yaw _returnvalue))) (.x ActionValue) false)
  (Pawn|Input|AddMovementInput (Math|Vector|GetForwardVector (Math|Rotator|MakeRotator 0.0 0.0 (.yaw (Pawn|GetControlRotation :!class /Script/Engine.Pawn)))) (.y ActionValue) false))

(event EventBeginPlay
  (CallFunction|SetPath)
  (CallFunction|SplineMovement)
  (bind _asplayer_controller (Utilities|Casting|CastToPlayerController (Game|GetPlayerController 0)))
  (Utilities|IsValid (PlayerController|LocalPlayerSubsystems|GetEnhancedInputLocalPlayerSubsystem _asplayer_controller)
    (:Is%20Valid
      (Input|AddMappingContext (PlayerController|LocalPlayerSubsystems|GetEnhancedInputLocalPlayerSubsystem _asplayer_controller) "/Game/Starfox/Inputs/IMC_PlayerInputs.IMC_PlayerInputs" 0 "(bIgnoreAllPressedKeysUntilRelease=True,bForceImmediately=False,bNotifyUserSettings=False)"))))

(fn ConstructionScript)

(fn SetPath
  (bind _outactors (Actor|GetAllActorswithTag "Fligth_path"))
  (bind _asbp_spline_path (Utilities|Casting|CastToBP_SplinePath (Utilities|Array|Get(acopy) _outactors))
    (:then
      (Variables|Default|SetSpline%20to%20follow _asbp_spline_path))
    (:CastFailed
      (Development|PrintText "Spline not found"))))