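; Starfox-style aiming target that rides a spline on rails, follows the mouse and spawns bullets on Space.
; A Speed-scaled timeline sets its spline transform, offsets the capsule along the camera's forward vector, then clamps the cursor within TargetBounds.
; Tick also lerps actor location toward a bounds-scaled mouse position in world XY, competing with the spline movement.
; BeginPlay shows the cursor, deactivates its camera and starts the movement.
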(event Custom|move%20On%20Spline
  (bind _splinereference (Variables|Default|GetSplineReference))
  (bind _spline (Variables|/Game/Starfox/BluePrints/BP_SplinePath.BP_SplinePath_C|GetSpline _splinereference))
  (Components|Timeline|SetPlayRate (Variables|Default|GetTimeline) (/ 1.0 (Variables|Default|GetSpeed)))
  (bind _newtrack_0 (Timeline|Timeline Play)
    (:Update
      (Variables|Default|Setcurrent%20distance%20on%20spline (Math|Float|Lerp 0.0 (Spline|GetSplineLength _spline) _newtrack_0))
      (Transformation|SetActorLocationAndRotation (Spline|GetLocationatDistanceAlongSpline _spline (Math|Float|Lerp 0.0 (Spline|GetSplineLength _spline) _newtrack_0) "World") (Spline|GetRotationatDistanceAlongSpline _spline (Math|Float|Lerp 0.0 (Spline|GetSplineLength _spline) _newtrack_0) "World"))
      (target|UpdateTarget))))

(event EventBeginPlay
  (bind _returnvalue (Game|GetPlayerController 0))
  (Variables|/Script/Engine.PlayerController|SetbShowMouseCursor _returnvalue true)
  (Input|SetInputModeGameandUI _returnvalue 0 "DoNotLock" true false)
  (Components|Activation|SetActive (Variables|Default|GetCameraComponent) false false)
  (CallFunction|MoveonSpline))

(event EventTick
  (params (DeltaSeconds :type Float%20%28single-precision%29))
  (bind _returnvalue (Game|GetPlayerController 0))
  (bind _returnvalue_2 (Viewport|GetViewportSize))
  (bind _target_bounds (Variables|Default|GetTarget%20Bounds))
  (bind (_locationx _locationy) (Game|Player|GetMousePosition _returnvalue))
  (bind (_x _y) (Math|Vector2D|BreakVector2D _returnvalue_2))
  (bind (_x_2 _y_2) (Math|Vector|BreakVector _target_bounds))
  (bind _output_get (Variables|Default|Setnormalized%20X (* (- (/ _locationx _x) 0.5) 2.0)))
  (bind _output_get_2 (Variables|Default|Setnormalized%20Y (* (- (/ _y _locationy) 0.5) 2.0)))
  (bind _output_get_3 (Variables|Default|Settarget%20location (Math|Vector|MakeVector (* _x_2 _output_get) (* _output_get_2 _y_2) 0.0)))
  (Transformation|SetActorLocation (Math|Vector|Lerp(Vector) (Transformation|GetActorLocation) _output_get_3 DeltaSeconds) false false))

(event Input|KeyboardEvents|SpaceBar
  (params (Key :type Key%20Structure))
  (:Pressed
    (Game|SpawnActorfromClass "/Game/Starfox/BluePrints/Bullet.Bullet_C" (Transformation|GetWorldTransform (Variables|Default|GetShooting%20spawn)) "AlwaysSpawn" "MultiplyWithRoot" 0 0)))

(fn ConstructionScript)

(fn UpdateTarget
  (Transformation|SetWorldLocation (Variables|Default|GetCapsuleComponent) (+ (Transformation|GetWorldLocation (Variables|Default|GetCapsuleComponent)) (* (Math|Vector|GetForwardVector (Variables|Default|GetCameraComponent)) (Variables|Default|GetTarget%20Distance))) false false)
  (CallFunction|CheckBounds))

(fn CheckBounds
  (bind _returnvalue (Game|GetPlayerController 0))
  (bind _returnvalue_2 (Viewport|GetViewportSize))
  (bind _target_bounds (Variables|Default|GetTarget%20Bounds))
  (bind (_locationx _locationy) (Game|Player|GetMousePosition _returnvalue))
  (bind _returnvalue_3 (- "1.000000,1.000000,0.000000" _target_bounds))
  (bind _returnvalue_4 (* _returnvalue_3 _returnvalue_2))
  (bind _returnvalue_5 (/ _returnvalue_4 "2.000000,2.000000,0.000000"))
  (bind (_x _y) (Math|Vector2D|BreakVector2D _returnvalue_5))
  (bind _returnvalue_6 (- _returnvalue_2 _returnvalue_5))
  (bind (_x_2 _y_2) (Math|Vector2D|BreakVector2D _returnvalue_6))
  (Utilities|FlowControl|Sequence
    (:then_0
      (LocalVariables|SetOut%20of%20bounds%20right (> _locationx _x_2))
      (LocalVariables|Setout%20of%20bounds%20left (< _locationx _x))
      (LocalVariables|Setout%20of%20bounds%20down (> _locationy _y_2))
      (LocalVariables|SetOut%20of%20bounds%20up (< _locationy _y))
      (LocalVariables|SetMinBoundXY (Math|Conversions|ToVector(Vector2D) _returnvalue_5))
      (LocalVariables|SetMaxBoundXY (Math|Conversions|ToVector(Vector2D) _returnvalue_6))
      (LocalVariables|Setcurrent%20position (Math|Vector|MakeVector _locationx _locationy 0.0)))
    (:then_1
      (if (LocalVariables|GetOut%20of%20bounds%20right)
        (Class|PlayerController|SetMouseLocation (Game|GetPlayerController 0) (Math|Float|Truncate (.X (Math|Vector|BreakVector (LocalVariables|GetMaxBoundXY)))) (Math|Float|Truncate (.Y (Math|Vector|BreakVector (LocalVariables|Getcurrent%20position)))))))
    (:then_2
      (if (LocalVariables|Getout%20of%20bounds%20left)
        (Class|PlayerController|SetMouseLocation (Game|GetPlayerController 0) (Math|Float|Truncate (.X (Math|Vector|BreakVector (LocalVariables|GetMinBoundXY)))) (Math|Float|Truncate (.Y (Math|Vector|BreakVector (LocalVariables|Getcurrent%20position)))))))
    (:then_3
      (if (LocalVariables|GetOut%20of%20bounds%20up)
        (Class|PlayerController|SetMouseLocation (Game|GetPlayerController 0) (Math|Float|Truncate (.X (Math|Vector|BreakVector (LocalVariables|Getcurrent%20position)))) (Math|Float|Truncate (.Y (Math|Vector|BreakVector (LocalVariables|GetMinBoundXY)))))))
    (:then_4
      (if (LocalVariables|Getout%20of%20bounds%20down)
        (Class|PlayerController|SetMouseLocation (Game|GetPlayerController 0) (Math|Float|Truncate (.X (Math|Vector|BreakVector (LocalVariables|Getcurrent%20position)))) (Math|Float|Truncate (.Y (Math|Vector|BreakVector (LocalVariables|GetMaxBoundXY)))))))))