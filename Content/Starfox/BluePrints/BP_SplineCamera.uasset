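; Spline-following camera actor for the Starfox game that travels along a referenced spline on rails.
; On BeginPlay it starts a timeline whose play rate is scaled so the trip takes a configurable completion time.
; Each update maps the timeline alpha to distance along the spline, applying that world location minus an offset and the spline's rotation.
; Tick looks up the spaceship actor but does nothing with the result.
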(event Custom|Move%20object
  (bind _spline_to_follow (Variables|Default|GetSpline%20To%20Follow))
  (bind _spline (Variables|/Game/Starfox/BluePrints/BP_SplinePath.BP_SplinePath_C|GetSpline _spline_to_follow))
  (Components|Timeline|SetPlayRate (Variables|Default|GetT_Move) (/ 1.0 (Variables|Default|GetTIme%20To%20Complete)))
  (bind _move_track (Timeline|T_Move Play)
    (:Update
      (Transformation|SetActorLocationAndRotation (- (Spline|GetLocationatDistanceAlongSpline _spline (Math|Float|Lerp 0.0 (Spline|GetSplineLength _spline) _move_track) "World") (Variables|Default|Getoffet)) (Spline|GetRotationatDistanceAlongSpline _spline (Math|Float|Lerp 0.0 (Spline|GetSplineLength _spline) _move_track) "World")))))

(event EventBeginPlay
  (CallFunction|MoveObject))

(event Collision|EventActorBeginOverlap
  (params (OtherActor :type Actor%20Object%20Reference)))

(event EventTick
  (params (DeltaSeconds :type Float%20%28single-precision%29))
  (Actor|GetActorOfClass "/Game/Starfox/BluePrints/SpaceShipBluePrint.SpaceShipBluePrint_C"))

(fn ConstructionScript)