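; BP_target is an actor that moves itself along a spline path when play begins.
; BeginPlay takes the first BP_SplinePath found in the level and starts MoveOnSpline.
; A timeline track is lerped across the spline length, setting the actor's world location and rotation on each update.
; The timeline's play rate is the inverse of ForwardSpeed, so a higher value means slower travel.
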(event Custom|MoveOnSpline
  (bind _splinereference (Variables|Default|GetSplineReference))
  (bind _spline (Variables|/Game/NewFolder/BluePrints/BP_SplinePath.BP_SplinePath_C|GetSpline _splinereference))
  (Components|Timeline|SetPlayRate (Variables|Default|GetT_move) (/ 1.0 (Variables|Default|GetForwardSpeed)))
  (bind _move_track (Timeline|T_move Play)
    (:Update
      (Transformation|SetActorLocationAndRotation (Spline|GetLocationatDistanceAlongSpline _spline (Math|Float|Lerp 0.0 (Spline|GetSplineLength _spline) _move_track) "World") (Spline|GetRotationatDistanceAlongSpline _spline (Math|Float|Lerp 0.0 (Spline|GetSplineLength _spline) _move_track) "World")))))

(event EventBeginPlay
  (bind _outactors (Actor|GetAllActorsOfClass "/Game/NewFolder/BluePrints/BP_SplinePath.BP_SplinePath_C"))
  (Variables|Default|SetSplineReference (Utilities|Array|Get(acopy) _outactors))
  (CallFunction|MoveonSpline))

(event Collision|EventActorBeginOverlap
  (params (OtherActor :type Actor%20Object%20Reference)))

(event EventTick
  (params (DeltaSeconds :type Float%20%28single-precision%29)))

(fn ConstructionScript)