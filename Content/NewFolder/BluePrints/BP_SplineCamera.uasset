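; BP_SplineCamera is an actor, by its name a camera, that flies along another actor's spline starting at BeginPlay.
; A timeline, its play rate set to the inverse of TimeToComplete, outputs a FlightTrack alpha that is lerped to a distance along SplineToFollow's spline.
; Each update sets the actor's location from that distance in world space and its rotation in local space.
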(event Custom|Spline%20movement
  (bind _spline_to_follow (Variables|Default|GetSpline%20to%20follow))
  (bind _spline (Variables|/Game/NewFolder/BluePrints/BP_SplinePath.BP_SplinePath_C|GetSpline _spline_to_follow))
  (Components|Timeline|SetPlayRate (Variables|Default|GetTimeline) (/ 1.0 (Variables|Default|GetTime%20to%20complete)))
  (bind _flight_track (Timeline|Timeline Play)
    (:Update
      (Transformation|SetActorLocationAndRotation (Spline|GetLocationatDistanceAlongSpline _spline (Math|Float|Lerp 0.0 (Spline|GetSplineLength _spline) _flight_track) "World") (Spline|GetRotationatDistanceAlongSpline _spline (Math|Float|Lerp 0.0 (Spline|GetSplineLength _spline) _flight_track) "Local")))))

(event EventBeginPlay
  (CallFunction|SplineMovement))

(event Collision|EventActorBeginOverlap
  (params (OtherActor :type Actor%20Object%20Reference)))

(event EventTick
  (params (DeltaSeconds :type Float%20%28single-precision%29)))

(fn ConstructionScript)